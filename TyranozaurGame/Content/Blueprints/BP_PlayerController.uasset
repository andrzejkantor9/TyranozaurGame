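; Player controller that lets the player drag cubes around the level with the mouse cursor.
; Grab traces under the cursor and picks up any actor whose display name contains "cube", printing the hit for debugging.
; While held, Tick re-traces and moves it to the hit's X/Y, at a height captured only on the first successful grab via DoOnce.
; ZoomIn is an empty stub, with unconnected height-adjustment nodes left over.
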(event EventTick
  (params (DeltaSeconds :type Float%20%28single-precision%29))
  (bind _returnvalue (Game|GetPlayerController 0))
  (bind (_worldlocation _worlddirection) (Game|Player|ConvertMouseLocationToWorldSpace _returnvalue))
  (if (Variables|Default|GetMoveCube)
    (bind _outhit (Collision|LineTraceByChannel _worldlocation (+ _worldlocation (* _worlddirection 2e+03)) "TraceTypeQuery1" false 0 "None"))
    (Transformation|SetActorLocation (Variables|Default|GetMovedCube) (Math|Vector|MakeVector (.X (Math|Vector|BreakVector (.Location (Collision|BreakHitResult _outhit)))) (.Y (Math|Vector|BreakVector (.Location (Collision|BreakHitResult _outhit)))) (Variables|Default|GetCubeZLocation)) false false)))

(event Input|ActionEvents|InputActionGrab
  (params (Key :type Key%20Structure :default "None"))
  (bind _returnvalue (Game|GetPlayerController 0))
  (bind (_worldlocation _worlddirection) (Game|Player|ConvertMouseLocationToWorldSpace _returnvalue))
  ;[1 1 1] Grab
  (:Pressed
    (bind _outhit (Collision|LineTraceByChannel _worldlocation (+ _worldlocation (* _worlddirection 2e+03)) "TraceTypeQuery1" false 0 "None"))
    (Development|PrintString (Utilities|String|Append "Hit cube: " (Utilities|GetDisplayName (.HitActor (Collision|BreakHitResult _outhit))) ", location: " (Utilities|String|ToString(Vector) (.Location (Collision|BreakHitResult _outhit)))))
    (if (Utilities|String|Contains (Utilities|GetDisplayName (.HitActor (Collision|BreakHitResult _outhit))) "cube")
      (Variables|Default|SetMoveCube true)
      (Variables|Default|SetMovedCube (.HitActor (Collision|BreakHitResult _outhit)))
      (Utilities|FlowControl|DoOnce false
        (:Completed
          (Variables|Default|SetCubeZLocation (.Z (Math|Vector|BreakVector (.Location (Collision|BreakHitResult _outhit)))))))
      (else
        (Variables|Default|SetMoveCube false))))
  (:Released
    (Variables|Default|SetMoveCube false)))

(event Input|ActionEvents|InputActionZoomIn
  (params (Key :type Key%20Structure :default "None")))

(event Input|ActionEvents|InputActionZoomOut
  (params (Key :type Key%20Structure :default "None")))

(event Input|AxisEvents|InputAxisZoomIn
  (params (AxisValue :type Float%20%28single-precision%29)))

(fn ConstructionScript)